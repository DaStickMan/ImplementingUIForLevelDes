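; BP_Barricade is an interactable barricade made of four board meshes that collapses when interacted with.
; On the interact event it enables physics simulation on the boards and wakes their rigid bodies so they can fall.
; After a short delay it disables the boards' collision and calls OnBarricadeRemoved to signal that the barricade is cleared.
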(event EventStartEventsonInteract
  (Physics|SetSimulatePhysics (Variables|Default|GetSM_Boards1) true)
  (Class|PrimitiveComponent|WakeAllRigidBodies (Variables|Default|GetSM_Boards))
  (Utilities|FlowControl|Delay 2.0)
  (Collision|SetCollisionEnabled (Variables|Default|GetSM_Boards) "NoCollision")
  (Default|CallOnBarricadeRemoved))

(fn ConstructionScript
  (|CallParentFunction))