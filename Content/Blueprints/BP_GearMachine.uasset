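; BP_GearMachine is an interactable machine that takes a gear, which stays hidden from BeginPlay until a successful interaction.
; Interacting while locked shows the locked text on the interact UI; otherwise it reveals the gear mesh, hides the UI and calls GearMachineStarted.
; The locked event calls InspectGearMachine, and the construction script only runs the parent's.
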(event EventStartEventsonLocked
  (Class|InteractiveSwitchActor|InspectGearMachine))

(event EventBeginPlay
  (Development|SetHiddeninGame (Variables|Default|GetSM_Gear) true false))

(event EventStartEventsonInteract
  (if (Variables|Default|GetIsLocked)
    (Rendering|Components|TextRender|SetText (Variables|Default|GetInteractUI) (Variables|Default|GetLocked%20Text))
    (else
      (Development|SetHiddeninGame (Variables|Default|GetSM_Gear) false false)
      (Development|SetHiddeninGame (Variables|Default|GetInteractUI) true false)
      (Class|InteractiveSwitchActor|GearMachineStarted))))

(fn ConstructionScript
  (|CallParentFunction))