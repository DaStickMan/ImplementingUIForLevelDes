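; Base interactable actor Blueprint that handles lockable, one-time interactions with a text prompt.
; The InteractRadius overlap shows or hides InteractUI until the interaction completes.
; Interact either shows the locked text or marks completion and hides the prompt, then calls overridable locked or interact events for children.
; Unlock clears the lock and switches the prompt to the unlocked text.
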(event OnComponentBeginOverlap(InteractRadius)
  (params (OverlappedComponent :type Primitive%20Component%20Object%20Reference) (OtherActor :type Actor%20Object%20Reference) (OtherComp :type Primitive%20Component%20Object%20Reference) (OtherBodyIndex :type Integer) (bFromSweep :type Boolean) (SweepResult :type Hit%20Result%20Structure%20%28by%20ref%29))
  (if (not (Variables|BPInteractive|GetInteractComplete))
    ;[0.5208 0.5208 0.5208 0.5 40] EXISTING UI
    ; TEXT RENDER
    (Development|SetHiddeninGame (Variables|Default|GetInteractUI) false false)))

(event OnComponentEndOverlap(InteractRadius)
  (params (OverlappedComponent :type Primitive%20Component%20Object%20Reference) (OtherActor :type Actor%20Object%20Reference) (OtherComp :type Primitive%20Component%20Object%20Reference) (OtherBodyIndex :type Integer))
  (if (not (Variables|BPInteractive|GetInteractComplete))
    ;[0.5208 0.5208 0.5208 0.5 40] EXISTING UI
    ; TEXT RENDER
    (Development|SetHiddeninGame (Variables|Default|GetInteractUI) true false)))

(event Custom|StartEventsOnInteract)

(event Custom|StartEventsOnLocked)

(event EventUnlock
  (Variables|BP_Interactive|SetIsLocked false)
  (Rendering|Components|TextRender|SetText (Variables|Default|GetInteractUI) (Variables|BPInteractive|GetUnlocked%20Text)))

(event EventInteract
  (params (PlayerCharacter :type Ue%204ASP%20Character%20Object%20Reference))
  (bind _interactui (Variables|Default|GetInteractUI))
  (if (Variables|BP_Interactive|GetIsLocked)
    (Rendering|Components|TextRender|SetText _interactui (Variables|BPInteractive|GetLocked%20Text))
    (Development|SetHiddeninGame _interactui false false)
    (CallFunction|StartEventsonLocked)
    (else
      (Variables|BPInteractive|SetInteractComplete true)
      (Development|SetHiddeninGame (Variables|Default|GetInteractUI) true false)
      (CallFunction|StartEventsonInteract))))

(fn ConstructionScript)