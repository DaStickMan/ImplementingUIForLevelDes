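; Parent Blueprint for a key pickup that unlocks its assigned actors when the player interacts with it.
; Interact fires once, hiding the mesh and prompt text, disabling collision, and sending UnlockMessage to each ActorsToUnlock entry through BPI_Interaction.
; It then calls StartEventsOnTaken, an empty hook for children, while the InteractionRadius overlap toggles the text until the key is taken.
; The Construction Script removes valid entries lacking the interface from the list.
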(event OnComponentBeginOverlap(InteractionRadius)
  (params (OverlappedComponent :type Primitive%20Component%20Object%20Reference) (OtherActor :type Actor%20Object%20Reference) (OtherComp :type Primitive%20Component%20Object%20Reference) (OtherBodyIndex :type Integer) (bFromSweep :type Boolean) (SweepResult :type Hit%20Result%20Structure%20%28by%20ref%29))
  (if (not (Variables|6028BPKeyParent|GetIsTaken))
    (Development|SetHiddeninGame (Variables|Default|GetTextRender) false false)))

(event OnComponentEndOverlap(InteractionRadius)
  (params (OverlappedComponent :type Primitive%20Component%20Object%20Reference) (OtherActor :type Actor%20Object%20Reference) (OtherComp :type Primitive%20Component%20Object%20Reference) (OtherBodyIndex :type Integer))
  (if (not (Variables|6028BPKeyParent|GetIsTaken))
    (Development|SetHiddeninGame (Variables|Default|GetTextRender) true false)))

(event Custom|StartEventsOnTaken)

(event EventInteract
  (params (PlayerCharacter :type Ue%204ASP%20Character%20Object%20Reference))
  (Utilities|FlowControl|DoOnce false
    (:Completed
      (Variables|Default|SetPlayer%20Character PlayerCharacter) ; NOT NEEDED!!!
      (Variables|6028BPKeyParent|SetIsTaken true)
      (Development|SetHiddeninGame (Variables|Default|GetStaticMesh) true false)
      (Collision|SetActorEnableCollision self false)
      (for _array_element (Variables|6028BPKeyParent|GetActorsToUnlock)
        (if (Utilities|DoesObjectImplementInterface _array_element "/Game/Blueprints/FirstPersonTemplate/BPI_Interaction.BPI_Interaction_C")
          (Class|BPIInteraction|Unlock(Message) _array_element (Variables|Default|GetPlayer%20Character))))
      (CallFunction|StartEventsonTaken))))

(fn ConstructionScript
  (for _array_element (Variables|6028BPKeyParent|GetActorsToUnlock)
    (Utilities|IsValid _array_element
      (:Is%20Valid
        (if (not (Utilities|DoesObjectImplementInterface _array_element "/Game/Blueprints/FirstPersonTemplate/BPI_Interaction.BPI_Interaction_C"))
          (Utilities|Array|RemoveItem (Variables|6028BPKeyParent|GetActorsToUnlock) _array_element))))))