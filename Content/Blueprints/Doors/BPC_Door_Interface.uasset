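; Door Blueprint that handles player-style interaction, lock state and a text prompt.
; Interact shows locked text and broadcasts a locked event, or alternates OpenDoor and CloseDoor through a FlipFlop, toggling text visibility and broadcasting on open.
; Unlock clears the lock and updates the text.
; OpenDoorExternal jumps straight into either branch, bypassing the lock and FlipFlop state, and is noted for a later AI intro.
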(event Custom|OpenDoorExternal
  (params (Open :type Boolean))
  ;[0.1414 1 0 0.5] 6029 OPEN DOOR EXTERNAL (FOR AI INTRO LATER)
  (if Open
    (CallFunction|OpenDoor)
    (Development|SetHiddeninGame (Variables|Default|GetTextRender) true false)
    (Default|CallOnDoorOpened)
    (else
      (CallFunction|CloseDoor)
      (Development|SetHiddeninGame (Variables|Default|GetTextRender) false false))))

(event EventUnlock
  (Variables|Default|SetIsLocked false)
  (Rendering|Components|TextRender|SetText (Variables|Default|GetTextRender) (Variables|Default|GetIsUnlocked%20Text)))

(event EventInteract
  (params (PlayerCharacter :type Ue%204ASP%20Character%20Object%20Reference))
  (if (Variables|Default|GetIsLocked)
    (Rendering|Components|TextRender|SetText (Variables|Default|GetTextRender) (Variables|Default|GetIsLocked%20Text))
    (Class|ActorDoor|InteractLoked)
    (Default|CallOnDoorInteractLocked0)
    (else
      (Utilities|FlowControl|FlipFlop
        (:A
          (CallFunction|OpenDoor)
          (Development|SetHiddeninGame (Variables|Default|GetTextRender) true false)
          (Default|CallOnDoorOpened))
        (:B
          (CallFunction|CloseDoor)
          (Development|SetHiddeninGame (Variables|Default|GetTextRender) false false))))))

(fn ConstructionScript
  (|CallParentFunction))