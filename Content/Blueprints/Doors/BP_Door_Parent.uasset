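; Parent door Blueprint that supports single or double swinging doors, with a proximity text prompt and a lock state.
; The construction script uses DoubleDoor to remove unused door components and, for double doors, rescale the frame.
; OpenDoor and CloseDoor play or reverse the matching timeline to lerp door rotation.
; InteractionRadius overlaps toggle the prompt, while functions clear the lock and update its text, or toggle interaction collision.
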(event OnComponentBeginOverlap(InteractionRadius)
  (params (OverlappedComponent :type Primitive%20Component%20Object%20Reference) (OtherActor :type Actor%20Object%20Reference) (OtherComp :type Primitive%20Component%20Object%20Reference) (OtherBodyIndex :type Integer) (bFromSweep :type Boolean) (SweepResult :type Hit%20Result%20Structure%20%28by%20ref%29))
  ;[1 1 1 0.5] UI
  ;;[0.5208 0.5208 0.5208 0.5 40] EXISTING UI
  ;; TEXT RENDER
  (Development|SetHiddeninGame (Variables|Default|GetTextRender) false false))

(event OnComponentEndOverlap(InteractionRadius)
  (params (OverlappedComponent :type Primitive%20Component%20Object%20Reference) (OtherActor :type Actor%20Object%20Reference) (OtherComp :type Primitive%20Component%20Object%20Reference) (OtherBodyIndex :type Integer))
  ;[1 1 1 0.5] UI
  ;;[0.5208 0.5208 0.5208 0.5 40] EXISTING UI
  ;; TEXT RENDER
  (Development|SetHiddeninGame (Variables|Default|GetTextRender) true false))

(event Custom|OpenDoor
  ;[1 1 1] Door Animation
  (if (Variables|6028BPDoor|GetDoubleDoor)
    (bind _door_alpha (Timeline|DoorAnimation_Double Play)
      (:Update
        (Transformation|SetRelativeRotation (Variables|Default|GetDoor_L) (Math|Rotator|Lerp(Rotator) "0, 0, 0" "0,-110.000000, 0" _door_alpha true) false false)
        (Transformation|SetRelativeRotation (Variables|Default|GetDoor_R) (Math|Rotator|Lerp(Rotator) "0, 0, 0" "0,110.000000, 0" _door_alpha true) false false)))
    (else
      (bind _door_alpha_2 (Timeline|DoorAnimation Play)
        (:Update
          (Transformation|SetRelativeRotation (Variables|Default|GetDoor_Single) (Math|Rotator|Lerp(Rotator) "0, 0, 0" "0,-110.000000, 0" _door_alpha_2 true) false false))))))

(event Custom|CloseDoor
  ;[1 1 1] Door Animation
  (if (Variables|6028BPDoor|GetDoubleDoor)
    (bind _door_alpha (Timeline|DoorAnimation_Double Reverse)
      (:Update
        (Transformation|SetRelativeRotation (Variables|Default|GetDoor_L) (Math|Rotator|Lerp(Rotator) "0, 0, 0" "0,-110.000000, 0" _door_alpha true) false false)
        (Transformation|SetRelativeRotation (Variables|Default|GetDoor_R) (Math|Rotator|Lerp(Rotator) "0, 0, 0" "0,110.000000, 0" _door_alpha true) false false)))
    (else
      (bind _door_alpha_2 (Timeline|DoorAnimation Reverse)
        (:Update
          (Transformation|SetRelativeRotation (Variables|Default|GetDoor_Single) (Math|Rotator|Lerp(Rotator) "0, 0, 0" "0,-110.000000, 0" _door_alpha_2 true) false false))))))

(fn ConstructionScript
  (if (Variables|6028BPDoor|GetDoubleDoor)
    (Components|DestroyComponent (Variables|Default|GetDoor_Single))
    (Transformation|SetRelativeScale3D (Variables|Default|GetDoorFrame) "1.250000,2.800000,1.150000")
    (else
      (Components|DestroyComponent (Variables|Default|GetDoor_L)))))

(fn UnlockDoor
  (Variables|6028_BP_Door|SetIsLocked false)
  (Rendering|Components|TextRender|SetText (Variables|Default|GetTextRender) (Variables|6028BPDoor|GetIsUnlocked%20Text)))

(fn 6029EnableInteraction
  (params (Enable :type Boolean))
  (bind _interactionradius (Variables|Default|GetInteractionRadius))
  (if Enable
    (Collision|SetCollisionEnabled _interactionradius "QueryAndPhysics")
    (else
      (Collision|SetCollisionEnabled _interactionradius "NoCollision"))))